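; BP_Customer is an AI customer that walks to the food stall, gets served and later leaves the level.
; On arrival it randomizes its health bar and fires ReadyToServe; BeginLeave shows a sick face, walks it to the exit, fires ReadyToExit and destroys it.
; Skeletal mesh is random; expressions swap materials on named face slots.
; DamageCustomer lowers health and triggers GameOver, subtracting damage again in its zero check.
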(event `self.ReceiveBeginPlay`
  (`self.SetupRandomMesh`)
  (bind _outactors (`GameplayStatics.GetAllActorsOfClass` "/Game/_Flubz/Blueprints/BP_FoodStall.BP_FoodStall_C"))
  (`|AIMoveTo` self (0.0 0.0 0.0) (`|GetArrayItem` _outactors)
    (:`OnSuccess`
      (`self.K2_SetActorRotation` (struct :`Yaw` -90.0))
      (bind _aswbp_health_bar (cast `/Game/_Flubz/Blueprints/Widgets/WBP_HealthBar` (`WidgetComponent.GetUserWidgetObject` (`self.HealthWidget`))))
      (bind _output_get (set `self.Health` (`KismetMathLibrary.RandomFloatInRange` 0.0 1.0)))
      (`ProgressBar.SetPercent` (`/Game/_Flubz/Blueprints/Widgets/WBP_HealthBar.HealthBar` _aswbp_health_bar) _output_get)
      (`self.ReadyToServe`))))

(event `BeginLeave`
  (`self.SetExpression` "NewEnumerator4")
  (`KismetSystemLibrary.Delay` 1.0)
  (bind _outactors (`GameplayStatics.GetAllActorsOfClass` "/Game/_Flubz/Blueprints/BP_ExitLocation.BP_ExitLocation_C"))
  (`|AIMoveTo` self (0.0 0.0 0.0) (`|GetArrayItem` _outactors)
    (:`OnSuccess`
      (`self.ReadyToExit`)
      (`self.K2_DestroyActor`))))

(fn `CustomerLeave`)

(fn `DamageCustomer`
  (params (DamageAmount :type "Float (double-precision)"))
  (bind _returnvalue (- (`self.Health`) (/ DamageAmount 100.0)))
  (bind _aswbp_health_bar (cast `/Game/_Flubz/Blueprints/Widgets/WBP_HealthBar` (`WidgetComponent.GetUserWidgetObject` (`self.HealthWidget`))))
  (bind _output_get (set `self.Health` _returnvalue))
  (`ProgressBar.SetPercent` (`/Game/_Flubz/Blueprints/Widgets/WBP_HealthBar.HealthBar` _aswbp_health_bar) _output_get)
  (if (<= _returnvalue 0.0)
    (bind _asbp_ld45player_controller_base (cast `/Game/_Flubz/Blueprints/BP_LD45PlayerControllerBase` (`GameplayStatics.GetPlayerController` 0)))
    (`/Game/_Flubz/Blueprints/BP_LD45PlayerControllerBase.GameOver` _asbp_ld45player_controller_base)))

(fn `Move`
  (params (Destination :type "Actor Object Reference")))

(fn `SetExpression`
  (params (NewExpression :type "/Game/_Flubz/Blueprints/Customer/EBP_CustomerExpression Enum" :default "NewEnumerator0"))
  (for (_array_element _array_index) (`MeshComponent.GetMaterialSlotNames` (`self.Mesh`))
    (if (or (== _array_element "Neutral1") (== _array_element "Neutral6"))
      (switch `/Game/_Flubz/Blueprints/Customer/EBP_CustomerExpression` NewExpression
        (:`NewEnumerator0`
          (set `self.CurrentExpressionElement` 0))
        (:`NewEnumerator1`
          (set `self.CurrentExpressionElement` 1))
        (:`NewEnumerator2`
          (set `self.CurrentExpressionElement` 2))
        (:`NewEnumerator3`
          (set `self.CurrentExpressionElement` 3))
        (:`NewEnumerator4`
          (set `self.CurrentExpressionElement` 4))
        (:`NewEnumerator5`
          (set `self.CurrentExpressionElement` 5)))
      (`PrimitiveComponent.SetMaterial` (`self.Mesh`) _array_index (`|GetArrayItem` (`self.ExpressionMaterials`) (`self.CurrentExpressionElement`))))))

(fn `SetupRandomMesh`
  (bind _output_get (set `self.RandomSkeletalMeshIndex` (`KismetMathLibrary.RandomInteger` 2)))
  (`SkinnedMeshComponent.SetSkinnedAssetAndUpdate` (`self.Mesh`) (`|GetArrayItem` (`self.CustomerMeshes`) _output_get) true))

(fn `UserConstructionScript`)