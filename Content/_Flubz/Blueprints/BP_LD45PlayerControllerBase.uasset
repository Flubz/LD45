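; Base player controller for a sandwich-serving game, tracking the current customer and the sandwich being built.
; A spawn event gets the next customer from the first BP_CustomerSpawner, while BeginPlay binds to the current customer's ready-to-serve event.
; Adding a recipe records it and spawns a part actor with its mesh at BP_SandwichSpawnLocation; clearing destroys those parts.
; Customer-ready, customer-left and sell-sandwich events are empty stubs.
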(event `OnSpawnNextCustomer`
  (bind _outactors (`GameplayStatics.GetAllActorsOfClass` "/Game/_Flubz/Blueprints/AI/BP_CustomerSpawner.BP_CustomerSpawner_C"))
  (bind _returnvalue (`/Game/_Flubz/Blueprints/AI/BP_CustomerSpawner.SpawnNewCustomer` (`|GetArrayItem` _outactors)))
  (set `self.CurrentCustomer` _returnvalue))

(event `self.ReceiveBeginPlay`
  (add `/Game/_Flubz/Blueprints/AI/BP_Customer.ReadyToServe` (`self.CurrentCustomer`) (delegate `OnCustomerIsReady`)))

(event `OnCustomerIsReady`)

(event `OnCustomerLeft`)

(event `SellSandwich`)

(fn `AddToCurrentSandwich`
  (params (NewRecipe :type "ItemData Structure"))
  (`KismetArrayLibrary.Array_Add` (`self.CurrentSandwich`) NewRecipe)
  (bind _outactors (`GameplayStatics.GetAllActorsOfClass` "/Game/_Flubz/Blueprints/BP_SandwichSpawnLocation.BP_SandwichSpawnLocation_C"))
  (bind _returnvalue (`|SpawnActorFromClass` "/Game/_Flubz/Blueprints/BP_Sandwichpart.BP_Sandwichpart_C" (`self.GetTransform` (`|GetArrayItem` _outactors)) "Undefined" "OverrideRootScale" null null))
  (`StaticMeshComponent.SetStaticMesh` (`/Game/_Flubz/Blueprints/BP_Sandwichpart.StaticMesh` _returnvalue) (`.ItemMesh` (break `ItemData` NewRecipe)))
  (`KismetArrayLibrary.Array_Add` (`self.SandwichPart`) _returnvalue))

(fn `ClearSandwich`
  (bind _sandwichpart (`self.SandwichPart`))
  (`KismetArrayLibrary.Array_Clear` (`self.CurrentSandwich`))
  (for _array_element _sandwichpart
    (`self.K2_DestroyActor` _array_element))
  (`KismetArrayLibrary.Array_Clear` _sandwichpart))

(fn `UserConstructionScript`)